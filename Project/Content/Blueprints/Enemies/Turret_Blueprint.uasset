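; Enemy turret that sweeps its yaw across a field of view until it detects the player, then turns to track and fire.
; Tick runs a forward sphere trace, widened when targeting is unlimited; tracking also recenters the sweep.
; FireAtTarget spawns timer-limited projectiles with random yaw deviation.
; Damage other than EnemyDamageType lowers health, and at zero the turret plays an explosion sound and is destroyed.
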(event Custom|ReceiveBeginPlay_Copy)

(event EventAnyDamage
  (params (Damage :type Float%20%28single-precision%29) (DamageType :type Damage%20Type%20Object%20Reference) (InstigatedBy :type Controller%20Object%20Reference) (DamageCauser :type Actor%20Object%20Reference))
  ;[1 1 1] Apply damage
  (if (!= (Utilities|GetClass DamageType) "/Game/Blueprints/Enemies/EnemyDamageType.EnemyDamageType_C")
    (CallFunction|ApplyDamage (Math|Float|Floor Damage))))

(event EventBeginPlay
  ;[1 1 1] Event Begin
  (Variables|Default|Setm_health (Variables|Default|Getm_maxHealth))
  (Variables|Default|Setm_target (Game|Player|GetPlayerPawn 0))
  (Variables|Default|Setm_baseRotation (Transformation|GetActorRotation)))

(event EventTick
  (params (DeltaSeconds :type Float%20%28single-precision%29))
  (bind _returnvalue (Transformation|GetActorLocation))
  (bind _returnvalue_2 (Transformation|GetActorRotation))
  (bind _returnvalue_3 (Transformation|GetActorLocation))
  (bind _returnvalue_4 (Utilities|Time|GetWorldDeltaSeconds))
  (bind _returnvalue_5 (Transformation|GetActorRotation))
  (bind _returnvalue_6 (Transformation|GetActorLocation))
  (bind _returnvalue_7 (Transformation|GetActorRotation))
  (bind _m_target (Variables|Default|Getm_target))
  (bind _m_rotationspeed (Variables|Default|Getm_rotationSpeed))
  (bind _returnvalue_8 (Transformation|GetActorLocation _m_target))
  (bind _returnvalue_9 (Math|Rotator|FindLookatRotation _returnvalue_3 _returnvalue_8))
  (bind _returnvalue_10 (Math|Interpolation|RInterpTo (Math|Rotator|MakeRotator (.pitch _returnvalue_5) (.yaw _returnvalue_5) (.roll _returnvalue_5)) (Math|Rotator|MakeRotator (.pitch _returnvalue_5) (.yaw _returnvalue_9) (.roll _returnvalue_5)) _returnvalue_4 _m_rotationspeed))
  (Audio|PlaySoundatLocation "/Game/Audio/Effects/TurretSound_Cue.TurretSound_Cue" (Transformation|GetActorLocation))
  (Math|Float|CompareFloat (Variables|Default|Getm_fireTimer) 0.0
    (:>
      (Variables|Default|Setm_fireTimer (- (Variables|Default|Getm_fireTimer) (Utilities|Time|GetWorldDeltaSeconds))))
    (:==
      _)
    (:<
      _))
  ;[1 1 1] Rotation
  (if (Variables|Default|Getm_targetClose)
    _
    (elif (Variables|Default|Getm_rotatingRight)
      (Transformation|SetActorRotation (Math|Rotator|MakeRotator (.pitch (Math|Interpolation|RInterpTo (Math|Rotator|MakeRotator (.pitch _returnvalue_7) (.yaw _returnvalue_7) (.roll _returnvalue_7)) (Math|Rotator|MakeRotator (.pitch _returnvalue_7) (+ (.yaw (Variables|Default|Getm_baseRotation)) (Variables|Default|Getm_halfFieldOfView)) (.roll _returnvalue_7)) (Utilities|Time|GetWorldDeltaSeconds) (Variables|Default|Getm_rotationSpeed))) (.yaw (Math|Interpolation|RInterpTo (Math|Rotator|MakeRotator (.pitch _returnvalue_7) (.yaw _returnvalue_7) (.roll _returnvalue_7)) (Math|Rotator|MakeRotator (.pitch _returnvalue_7) (+ (.yaw (Variables|Default|Getm_baseRotation)) (Variables|Default|Getm_halfFieldOfView)) (.roll _returnvalue_7)) (Utilities|Time|GetWorldDeltaSeconds) (Variables|Default|Getm_rotationSpeed))) (.roll (Math|Interpolation|RInterpTo (Math|Rotator|MakeRotator (.pitch _returnvalue_7) (.yaw _returnvalue_7) (.roll _returnvalue_7)) (Math|Rotator|MakeRotator (.pitch _returnvalue_7) (+ (.yaw (Variables|Default|Getm_baseRotation)) (Variables|Default|Getm_halfFieldOfView)) (.roll _returnvalue_7)) (Utilities|Time|GetWorldDeltaSeconds) (Variables|Default|Getm_rotationSpeed)))))
      (Math|Float|CompareFloat (.yaw (Math|Interpolation|RInterpTo (Math|Rotator|MakeRotator (.pitch _returnvalue_7) (.yaw _returnvalue_7) (.roll _returnvalue_7)) (Math|Rotator|MakeRotator (.pitch _returnvalue_7) (+ (.yaw (Variables|Default|Getm_baseRotation)) (Variables|Default|Getm_halfFieldOfView)) (.roll _returnvalue_7)) (Utilities|Time|GetWorldDeltaSeconds) (Variables|Default|Getm_rotationSpeed))) (- (+ (.yaw (Variables|Default|Getm_baseRotation)) (Variables|Default|Getm_halfFieldOfView)) 1e+01)
        (:>
          (Variables|Default|Setm_rotatingRight false :!label _label))
        (:==
          (goto _label))
        (:<
          _))
      (else
        (Transformation|SetActorRotation (Math|Rotator|MakeRotator (.pitch (Math|Interpolation|RInterpTo (Math|Rotator|MakeRotator (.pitch _returnvalue_2) (.yaw _returnvalue_2) (.roll _returnvalue_2)) (Math|Rotator|MakeRotator (.pitch _returnvalue_2) (- (.yaw (Variables|Default|Getm_baseRotation)) (Variables|Default|Getm_halfFieldOfView)) (.roll _returnvalue_2)) (Utilities|Time|GetWorldDeltaSeconds) (Variables|Default|Getm_rotationSpeed))) (.yaw (Math|Interpolation|RInterpTo (Math|Rotator|MakeRotator (.pitch _returnvalue_2) (.yaw _returnvalue_2) (.roll _returnvalue_2)) (Math|Rotator|MakeRotator (.pitch _returnvalue_2) (- (.yaw (Variables|Default|Getm_baseRotation)) (Variables|Default|Getm_halfFieldOfView)) (.roll _returnvalue_2)) (Utilities|Time|GetWorldDeltaSeconds) (Variables|Default|Getm_rotationSpeed))) (.roll (Math|Interpolation|RInterpTo (Math|Rotator|MakeRotator (.pitch _returnvalue_2) (.yaw _returnvalue_2) (.roll _returnvalue_2)) (Math|Rotator|MakeRotator (.pitch _returnvalue_2) (- (.yaw (Variables|Default|Getm_baseRotation)) (Variables|Default|Getm_halfFieldOfView)) (.roll _returnvalue_2)) (Utilities|Time|GetWorldDeltaSeconds) (Variables|Default|Getm_rotationSpeed)))))
        (Math|Float|CompareFloat (.yaw (Math|Interpolation|RInterpTo (Math|Rotator|MakeRotator (.pitch _returnvalue_2) (.yaw _returnvalue_2) (.roll _returnvalue_2)) (Math|Rotator|MakeRotator (.pitch _returnvalue_2) (- (.yaw (Variables|Default|Getm_baseRotation)) (Variables|Default|Getm_halfFieldOfView)) (.roll _returnvalue_2)) (Utilities|Time|GetWorldDeltaSeconds) (Variables|Default|Getm_rotationSpeed))) (+ (- (.yaw (Variables|Default|Getm_baseRotation)) (Variables|Default|Getm_halfFieldOfView)) 1e+01)
          (:>
            _)
          (:==
            (Variables|Default|Setm_rotatingRight true :!label _label_2))
          (:<
            (goto _label_2))))))
  (if (Variables|Default|Getm_limitedTargeting)
    (Variables|Default|Setm_targetClose false)
    ;[1 1 1] Limited Targeting
    (bind _outhits (Class|KismetSystemLibrary|SphereTraceMultiNEW _returnvalue (+ _returnvalue (* (Math|Vector|Normalize (Transformation|GetActorForwardVector)) (Variables|Default|Getm_targetingDistance))) (Variables|Default|Getm_radiusSight) "TraceTypeQuery2" false 0 "None" true))
    (bind _array_element (Utilities|Array|ForEachLoopwithBreak _outhits :!label _label_3)
      (:LoopBody
        (Utilities|Casting|CastToFirstPersonCharacter (.HitActor (Collision|BreakHitResult _array_element)))
        (Variables|Default|Setm_targetClose true)
        (goto _label_3 Break))
      (:Completed
        _))
    (else
      (Variables|Default|Setm_targetClose false)
      ;[1 1 1] Unlimited Targeting
      (bind _outhits_2 (Class|KismetSystemLibrary|SphereTraceMultiNEW _returnvalue_6 (+ _returnvalue_6 (* (Math|Vector|Normalize (Transformation|GetActorForwardVector)) (Variables|Default|Getm_targetingDistance))) (+ (Variables|Default|Getm_targetingDistance) (Variables|Default|Getm_radiusSight)) "TraceTypeQuery2" false 0 "None" true))
      (bind _array_element_2 (Utilities|Array|ForEachLoopwithBreak _outhits_2 :!label _label_4)
        (:LoopBody
          (Utilities|Casting|CastToFirstPersonCharacter (.HitActor (Collision|BreakHitResult _array_element_2)))
          (Variables|Default|Setm_targetClose true)
          (goto _label_4 Break))
        (:Completed
          _))))
  ;[1 1 1] Rotation
  (if (Variables|Default|Getm_targetClose)
    (Transformation|SetActorRotation _returnvalue_10)
    (Variables|Default|Setm_baseRotation _returnvalue_10)
    (CallFunction|FireatTarget)))

(fn ConstructionScript)

(fn ApplyDamage
  (params (damage :type Integer :default 0))
  (bind _m_maxhealth (Variables|Default|Getm_maxHealth))
  (bind _output_get (Variables|Default|Setm_health (- (Variables|Default|Getm_health) damage)))
  (Math|Integer|CompareInt _output_get _m_maxhealth
    (:>
      (Variables|Default|Setm_health _m_maxhealth))
    (:<
      (Math|Integer|CompareInt _output_get 0
        (:==
          _)
        (:<
          _))
      (Audio|PlaySoundatLocation "/Game/Audio/Effects/ExplosionTurrets_Cue.ExplosionTurrets_Cue" (Transformation|GetActorLocation))
      (Actor|DestroyActor))))

(fn FireatTarget
  (bind _returnvalue (Transformation|GetActorLocation))
  (bind _returnvalue_2 (Transformation|GetActorRotation))
  (bind _m_shootingdeviation (Variables|Default|Getm_shootingDeviation))
  (bind (_pitch _yaw _roll) (Class|KismetMathLibrary|BreakRot _returnvalue_2))
  ;[1 1 1] Shooting
  (Math|Float|CompareFloat (Variables|Default|Getm_fireTimer) 0.0
    (:==
      _)
    (:<
      _))
  (Variables|Default|Setm_fireTimer (Variables|Default|Getm_fireRate))
  (bind _returnvalue_3 (Game|SpawnActorfromClass "/Game/Blueprints/Enemies/EnemyProjectile.EnemyProjectile_C" (Math|Transform|MakeTransform (+ _returnvalue (Math|Vector|RotateVector (Variables|Default|Getm_gunRotationOffset) _returnvalue_2)) (Class|KismetMathLibrary|MakeRot _pitch (Math|Random|RandomFloatinRange (- _yaw _m_shootingdeviation) (+ _yaw _m_shootingdeviation)) _roll) "1.000000,1.000000,1.000000") true 0))
  (Variables|/Game/Blueprints/Enemies/EnemyProjectile.EnemyProjectile_C|Setm_collisionDamage _returnvalue_3 (Variables|Default|Getm_shootingDamage))
  (Audio|PlaySoundatLocation "/Game/Audio/Effects/TurretShot_01_Cue.TurretShot_01_Cue" _returnvalue))