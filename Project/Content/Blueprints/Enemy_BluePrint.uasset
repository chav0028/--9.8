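; Enemy Blueprint that tracks health and destroys the actor when damage depletes it.
; Health starts at the maximum on BeginPlay, and AnyDamage passes floored damage to ApplyDamageEnemy.
; That function subtracts the damage, caps health at the maximum, and destroys the actor once health is zero or below.
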(event EventAnyDamage
  (params (Damage :type Float%20%28single-precision%29) (DamageType :type Damage%20Type%20Object%20Reference) (InstigatedBy :type Controller%20Object%20Reference) (DamageCauser :type Actor%20Object%20Reference))
  (CallFunction|ApplyDamageEnemy (Math|Float|Floor Damage)))

(event EventBeginPlay
  (Variables|Default|Setm_health (Variables|Default|Getm_maxhealth)))

(event EventActorBeginOverlap
  (params (OtherActor :type Actor%20Object%20Reference)))

(event EventTick
  (params (DeltaSeconds :type Float%20%28single-precision%29)))

(fn ConstructionScript)

(fn ApplyDamageEnemy
  (params (damage :type Integer :default 0))
  (bind _m_maxhealth (Variables|Default|Getm_maxHealth))
  (bind _output_get (Variables|Default|Setm_health (- (Variables|Default|Getm_health) damage)))
  (Math|Integer|CompareInt _output_get _m_maxhealth
    (:>
      (Variables|Default|Setm_health _m_maxhealth))
    (:<
      (Math|Integer|CompareInt _output_get 0
        (:==
          _)
        (:<
          _))
      (Actor|DestroyActor))))