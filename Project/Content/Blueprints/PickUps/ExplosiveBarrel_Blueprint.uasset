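; Explosive barrel that detonates when it takes PlayerDamage, dealing environmental radial damage with falloff.
; ExplodeBarrels fires a radial impulse, activates the explosion effect, plays sound, then hides the mesh and disables its collision.
; It then recursively detonates unexploded barrels within the damage radius, with MExploded set first to prevent repeat blasts.
; ExplodeObject is a similar non-chaining variant whose only call here never runs.
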(event EventBeginPlay)

(event EventActorBeginOverlap
  (params (OtherActor :type Actor%20Object%20Reference)))

(event EventTick
  (params (DeltaSeconds :type Float%20%28single-precision%29)))

(event EventAnyDamage
  (params (Damage :type Float%20%28single-precision%29) (DamageType :type Damage%20Type%20Object%20Reference) (InstigatedBy :type Controller%20Object%20Reference) (DamageCauser :type Actor%20Object%20Reference))
  (if (== (Utilities|GetClass DamageType) "/Game/Blueprints/PlayerDamage.PlayerDamage_C")
    (if (not (Variables|Default|Getm_exploded))
      (Utilities|IsValid DamageCauser
        (:Is%20Valid
          (CallFunction|ExplodeBarrels (Transformation|GetActorLocation DamageCauser) Damage DamageCauser))))))

(fn ConstructionScript)

(fn ExplodeObject
  (params (HurtOrigin :type Vector) (BarrelDamageTaken :type Float%20%28single-precision%29 :default 0.0) (DamageCauser :type Actor%20Object%20Reference))
  (Utilities|IsValid DamageCauser
    (:Is%20Valid
      (Variables|Default|Setm_exploded true)
      (Class|RadialForceComponent|FireImpulse (Variables|Default|GetRadiusImpulse))
      (Class|GameplayStatics|ApplyRadialDamagewithFalloff (Variables|Default|Getm_damageAmount) (Variables|Default|Getm_minimumDamage) (.Origin (Collision|GetComponentBounds (Variables|Default|GetRadiusImpulse))) 5e+01 (Variables|Default|Getm_damageRadius) 1.0 "/Game/Blueprints/EnviromentDamage.EnviromentDamage_C" 0 self 0 "ECC_Visibility")
      (Components|Activation|Activate (Variables|Default|GetExplosion) false)
      (Rendering|SetVisibility (Variables|Debug|GetStaticMeshComponent) false false)
      (Collision|SetCollisionEnabled (Variables|Debug|GetStaticMeshComponent) "NoCollision"))))

(fn ExplodeBarrels
  (params (Hurtorigin :type Vector) (BarrelDamage :type Float%20%28single-precision%29 :default 0.0) (DamageCauser :type Actor%20Object%20Reference))
  ;[1 1 1] Damage
  (Utilities|IsValid DamageCauser
    (:Is%20Valid
      (Variables|Default|Setm_exploded true)
      (Game|Damage|ApplyDamage self BarrelDamage 0 DamageCauser "/Game/Blueprints/EnviromentDamage.EnviromentDamage_C")
      (Class|RadialForceComponent|FireImpulse (Variables|Default|GetRadiusImpulse))
      (Class|GameplayStatics|ApplyRadialDamagewithFalloff (Variables|Default|Getm_damageAmount) (Variables|Default|Getm_minimumDamage) (.Origin (Collision|GetComponentBounds (Variables|Default|GetRadiusImpulse))) 0.0 (Variables|Default|Getm_damageRadius) 1.0 "/Game/Blueprints/EnviromentDamage.EnviromentDamage_C" 0 self 0 "ECC_Visibility")
      ;[1 1 1] Effects
      (Components|Activation|Activate (Variables|Default|GetExplosion) false)
      (Audio|PlaySoundatLocation "/Game/Audio/Effects/ExplosionBarrel.ExplosionBarrel" (Transformation|GetActorLocation))
      (Rendering|SetVisibility (Variables|Debug|GetStaticMeshComponent) false false)
      (Collision|SetCollisionEnabled (Variables|Debug|GetStaticMeshComponent) "NoCollision")
      ;[1 1 1] Explode other barrels
      (bind _outactors (Actor|GetAllActorsOfClass "ExplosiveBarrel_Blueprint_C"))
      (for _array_element _outactors
        (if (not (Variables|ExplosiveBarrel_Blueprint_C|Getm_exploded _array_element))
          (Math|Float|CompareFloat (Transformation|GetDistanceTo _array_element) (Variables|Default|Getm_damageRadius)
            (:==
              _)
            (:<
              _))
          (CallFunction|ExplodeBarrels _array_element (Transformation|GetWorldLocation) (Variables|Default|Getm_damageAmount) self))))))