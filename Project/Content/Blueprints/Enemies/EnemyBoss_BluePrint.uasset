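; Boss enemy that faces the player, alternates high and low special attacks, and flags the level as over when its health runs out.
; Tick uses a rest timer and delays to flash a warning light, then enable that side's indicator, which deals max-health damage to an overlapping player.
; A melee volume tracks player proximity, and BeginPlay passes the boss to its AI controller's blackboard.
; The half-health check for special attacks is disconnected.
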(event OnComponentBeginOverlap(BottomIndicator)
  (params (OtherActor :type Actor%20Object%20Reference) (OtherComp :type Primitive%20Component%20Object%20Reference) (OtherBodyIndex :type Integer) (bFromSweep :type Boolean) (SweepResult :type Hit%20Result%20Structure%20%28by%20ref%29))
  ;[1 1 1] Triggers
  (bind _asfirst_person_character (Utilities|Casting|CastToFirstPersonCharacter OtherActor))
  (Game|Damage|ApplyDamage _asfirst_person_character (Math|Conversions|ToFloat(Integer) (Variables|/Game/FirstPersonBP/Blueprints/FirstPersonCharacter.FirstPersonCharacter_C|Getm_maxHealth _asfirst_person_character)) 0 self "/Game/Blueprints/Enemies/EnemyDamageType.EnemyDamageType_C"))

(event OnComponentBeginOverlap(TopIndicator)
  (params (OtherActor :type Actor%20Object%20Reference) (OtherComp :type Primitive%20Component%20Object%20Reference) (OtherBodyIndex :type Integer) (bFromSweep :type Boolean) (SweepResult :type Hit%20Result%20Structure%20%28by%20ref%29))
  ;[1 1 1] Triggers
  (bind _asfirst_person_character (Utilities|Casting|CastToFirstPersonCharacter OtherActor))
  (Game|Damage|ApplyDamage _asfirst_person_character (Math|Conversions|ToFloat(Integer) (Variables|/Game/FirstPersonBP/Blueprints/FirstPersonCharacter.FirstPersonCharacter_C|Getm_maxHealth _asfirst_person_character)) 0 self "/Game/Blueprints/Enemies/EnemyDamageType.EnemyDamageType_C"))

(event OnComponentBeginOverlap(MeleeAttackRange)
  (params (OtherActor :type Actor%20Object%20Reference) (OtherComp :type Primitive%20Component%20Object%20Reference) (OtherBodyIndex :type Integer) (bFromSweep :type Boolean) (SweepResult :type Hit%20Result%20Structure%20%28by%20ref%29))
  ;[1 1 1] Meleee
  (Utilities|Casting|CastToFirstPersonCharacter OtherActor)
  (Variables|Default|Setm_playerInMeleeRange true))

(event OnComponentEndOverlap(MeleeAttackRange)
  (params (OtherActor :type Actor%20Object%20Reference) (OtherComp :type Primitive%20Component%20Object%20Reference) (OtherBodyIndex :type Integer))
  ;[1 1 1] Meleee
  (Utilities|Casting|CastToFirstPersonCharacter OtherActor)
  (Variables|Default|Setm_playerInMeleeRange false))

(event EventBeginPlay
  ;[1 1 1] Start
  (|CallParentFunction)
  (bind _returnvalue (AI|GetAIController self))
  (bind _asenemy_controller (Utilities|Casting|CastToEnemyController _returnvalue))
  (Default|SetBlackboardValues _asenemy_controller self)
  (Collision|SetCollisionEnabled (Variables|Default|GetBottomIndicator) "NoCollision")
  (Rendering|SetVisibility false false)
  (Collision|SetCollisionEnabled (Variables|Default|GetTopIndicator) "NoCollision")
  (Rendering|SetVisibility false false))

(event EventActorBeginOverlap
  (params (OtherActor :type Actor%20Object%20Reference)))

(event EventTick
  (params (DeltaSeconds :type Float%20%28single-precision%29))
  (bind _m_warningtime (Variables|Default|Getm_warningTime))
  ;[1 1 1] Update
  (Variables|Default|Setm_firingCooldown (- (Variables|Default|Getm_firingCooldown) 0.0))
  (CallFunction|FacePlayerLockedZAxis)
  (Audio|PlaySoundatLocation "/Game/Audio/Effects/RobotSound_01_Cue.RobotSound_01_Cue" (Transformation|GetActorLocation))
  (if (Variables|Default|Getm_specialAttackModeOn)
    (if (Variables|Default|Getm_specialAttackDown)
      (Utilities|FlowControl|Delay (Variables|Default|Getm_attacksDuration))
      (Variables|Default|Setm_specialAttackDown false)
      (Rendering|SetVisibility (Variables|Default|GetBottomLight) false false)
      (Collision|SetCollisionEnabled (Variables|Default|GetBottomIndicator) "NoCollision")
      (Rendering|SetVisibility false false)
      (else
        (Utilities|FlowControl|Delay (Variables|Default|Getm_attacksDuration))
        (Variables|Default|Setm_specialAttackDown true)
        (Rendering|SetVisibility (Variables|Default|GetTopLight) false false)
        (Collision|SetCollisionEnabled (Variables|Default|GetTopIndicator) "NoCollision")
        (Rendering|SetVisibility (Variables|Default|GetTopIndicator) false false)))
    (Variables|Default|Setm_timerRest (Variables|Default|Getm_restTime))
    (Variables|Default|Setm_specialAttackModeOn false)
    (else
      (bind _output_get (Variables|Default|Setm_timerRest (+ (Variables|Default|Getm_timerRest) (Utilities|Time|GetWorldDeltaSeconds))))
      (Math|Float|CompareFloat _output_get (Variables|Default|Getm_restTime)
        (:>
          _)
        (:==
          _))
      (Variables|Default|Setm_timerRest 0.0)
      (if (Variables|Default|Getm_specialAttackDown)
        (Rendering|SetVisibility (Variables|Default|GetBottomLight) true false)
        (Utilities|FlowControl|Delay _m_warningtime)
        (Collision|SetCollisionEnabled (Variables|Default|GetBottomIndicator) "QueryAndPhysics")
        (Rendering|SetVisibility true false)
        (Variables|Default|Setm_specialAttackModeOn true)
        (else
          (Rendering|SetVisibility (Variables|Default|GetTopLight) true false)
          (Utilities|FlowControl|Delay _m_warningtime)
          (Collision|SetCollisionEnabled (Variables|Default|GetTopIndicator) "QueryAndPhysics")
          (Rendering|SetVisibility (Variables|Default|GetTopIndicator) true false)
          (Variables|Default|Setm_specialAttackModeOn true))))))

(event EventAnyDamage
  (params (Damage :type Float%20%28single-precision%29) (DamageType :type Damage%20Type%20Object%20Reference) (InstigatedBy :type Controller%20Object%20Reference) (DamageCauser :type Actor%20Object%20Reference))
  (bind _returnvalue (Math|Float|Floor Damage))
  ;[1 1 1] Damage
  (Math|Integer|CompareInt (- (Variables|Default|Getm_health) _returnvalue) 0
    (:>
      _)
    (:==
      (bind _asfirst_person_game_mode (Utilities|Casting|CastToFirstPersonGameMode (Game|GetGameMode) :!label _label))
      (Variables|/Game/FirstPersonBP/Blueprints/FirstPersonGameMode.FirstPersonGameMode_C|Setm_LevelOver _asfirst_person_game_mode true))
    (:<
      (goto _label)))
  (CallFunction|ApplyDamageEnemy _returnvalue))

(fn ConstructionScript
  (|CallParentFunction))