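; Checkpoint actor that updates the player's respawn point when the first-person character overlaps it.
; On overlap it copies the character's current transform into the FirstPersonGameMode's SpawnTransform, so the saved point is where the player touched it, not the checkpoint's own location.
; It then shows "Checkpoint" on player 0's HUD and clears the text after a short delay.
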(event EventBeginPlay)

(event EventActorBeginOverlap
  (params (OtherActor :type Actor%20Object%20Reference))
  ;[1 1 1] Set transform for new spawn point
  (bind _asfirst_person_character (Utilities|Casting|CastToFirstPersonCharacter OtherActor))
  (bind _asfirst_person_game_mode (Utilities|Casting|CastToFirstPersonGameMode (Game|GetGameMode)))
  (Variables|/Game/FirstPersonBP/Blueprints/FirstPersonGameMode.FirstPersonGameMode_C|SetSpawnTransform _asfirst_person_game_mode (Transformation|GetActorTransform _asfirst_person_character))
  (bind _asfirst_person_character_2 (Utilities|Casting|CastToFirstPersonCharacter (Game|GetPlayerCharacter 0)))
  (Variables|/Game/HUD_Elements/AntigravityGameHUD.AntigravityGameHUD_C|Setm_checkpointText (Variables|/Game/FirstPersonBP/Blueprints/FirstPersonCharacter.FirstPersonCharacter_C|Getm_playerHud _asfirst_person_character_2) "Checkpoint")
  (Utilities|FlowControl|Delay 1.0)
  (Variables|/Game/HUD_Elements/AntigravityGameHUD.AntigravityGameHUD_C|Setm_checkpointText (Variables|/Game/FirstPersonBP/Blueprints/FirstPersonCharacter.FirstPersonCharacter_C|Getm_playerHud _asfirst_person_character_2) ""))

(event EventTick
  (params (DeltaSeconds :type Float%20%28single-precision%29)))

(fn ConstructionScript)