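; Enemy robot base logic that tracks the player, takes non-enemy damage and explodes at zero health.
; Tick turns it toward a living player within targeting range, plays a robot sound and counts down the firing cooldown.
; FireAtTarget damages the player directly inside the melee overlap, otherwise spawning a projectile with random yaw deviation.
; FireAtTarget and the yaw-only FacePlayerLockedZAxis are defined but not called here.
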(event OnComponentBeginOverlap(MeleeAttackRange)
  (params (OtherActor :type Actor%20Object%20Reference) (OtherComp :type Primitive%20Component%20Object%20Reference) (OtherBodyIndex :type Integer) (bFromSweep :type Boolean) (SweepResult :type Hit%20Result%20Structure%20%28by%20ref%29))
  (Utilities|Casting|CastToFirstPersonCharacter OtherActor)
  (Variables|Default|Setm_playerInMeleeRange true))

(event OnComponentEndOverlap(MeleeAttackRange)
  (params (OtherActor :type Actor%20Object%20Reference) (OtherComp :type Primitive%20Component%20Object%20Reference) (OtherBodyIndex :type Integer))
  (Utilities|Casting|CastToFirstPersonCharacter OtherActor)
  (Variables|Default|Setm_playerInMeleeRange false))

(event EventAnyDamage
  (params (Damage :type Float%20%28single-precision%29) (DamageType :type Damage%20Type%20Object%20Reference) (InstigatedBy :type Controller%20Object%20Reference) (DamageCauser :type Actor%20Object%20Reference))
  (if (!= (Utilities|GetClass DamageType) "/Game/Blueprints/Enemies/EnemyDamageType.EnemyDamageType_C")
    (Utilities|IsValid self
      (:Is%20Valid
        (CallFunction|ApplyDamageEnemy (Math|Float|Floor Damage))))))

(event EventTick
  (params (DeltaSeconds :type Float%20%28single-precision%29))
  (CallFunction|FacePlayer)
  (Audio|PlaySoundatLocation "/Game/Audio/Effects/RobotSound_01_Cue.RobotSound_01_Cue" (Transformation|GetActorLocation))
  (Variables|Default|Setm_firingCooldown (- (Variables|Default|Getm_firingCooldown) DeltaSeconds)))

(event EventBeginPlay
  (Variables|Default|Setm_health (Variables|Default|Getm_maxhealth)))

(fn ConstructionScript)

(fn ApplyDamageEnemy
  (params (damage :type Integer :default 0))
  (bind _m_maxhealth (Variables|Default|Getm_maxHealth))
  (bind _output_get (Variables|Default|Setm_health (- (Variables|Default|Getm_health) damage)))
  (Math|Integer|CompareInt _output_get _m_maxhealth
    (:>
      (Variables|Default|Setm_health _m_maxhealth))
    (:<
      (Math|Integer|CompareInt _output_get 0
        (:==
          _)
        (:<
          _))
      (Audio|PlaySoundatLocation "/Game/Audio/Effects/ExplosionEnemies_Cue.ExplosionEnemies_Cue" (Transformation|GetActorLocation))
      (Actor|DestroyActor))))

(fn FacePlayer
  (bind _returnvalue (Transformation|GetActorLocation))
  (bind _returnvalue_2 (Transformation|GetActorRotation))
  (bind _returnvalue_3 (Game|Player|GetPlayerPawn 0))
  (bind _returnvalue_4 (Transformation|GetActorLocation _returnvalue_3))
  (bind _returnvalue_5 (Math|Rotator|FindLookatRotation _returnvalue _returnvalue_4))
  ;[1 1 1] Rotate Toward player direction
  (if (<= (Math|Vector|VectorLength (- _returnvalue _returnvalue_4)) (Variables|Default|Getm_targetingDistance))
    (bind _asfirst_person_game_mode (Utilities|Casting|CastToFirstPersonGameMode (Game|GetGameMode)))
    (if (not (Variables|/Game/FirstPersonBP/Blueprints/FirstPersonGameMode.FirstPersonGameMode_C|Getm_playerDead _asfirst_person_game_mode))
      (Utilities|IsValid (Variables|/Game/FirstPersonBP/Blueprints/FirstPersonGameMode.FirstPersonGameMode_C|Getm_player _asfirst_person_game_mode)
        (:Is%20Valid
          (Utilities|IsValid (Game|Player|GetPlayerPawn 0)
            (:Is%20Valid
              (Transformation|SetActorRotation (Math|Interpolation|RInterpTo (Math|Rotator|MakeRotator (.pitch _returnvalue_2) (.yaw _returnvalue_2) (.roll _returnvalue_2)) (Math|Rotator|MakeRotator (.pitch _returnvalue_5) (.yaw _returnvalue_5) (.roll _returnvalue_5)) 0.1 0.5)))))))))

(fn FireatTarget
  (bind _returnvalue (Transformation|GetActorLocation))
  (bind _returnvalue_2 (Transformation|GetActorRotation))
  (bind _m_shootingaccuracy (Variables|Default|Getm_shootingAccuracy))
  (bind _m_shootingdamage (Variables|Default|Getm_shootingDamage))
  (bind (_pitch _yaw _roll) (Class|KismetMathLibrary|BreakRot _returnvalue_2))
  ;[1 1 1] Shooting
  (Math|Float|CompareFloat (Variables|Default|Getm_firingCooldown) 0.0
    (:==
      _)
    (:<
      _))
  (Variables|Default|Setm_firingCooldown (Variables|Default|Getm_fireRate))
  (if (Variables|Default|Getm_playerInMeleeRange)
    (bind _asfirst_person_character (Utilities|Casting|CastToFirstPersonCharacter (Game|Player|GetPlayerPawn 0)))
    (Default|ApplyDamagePlayer _asfirst_person_character (Math|Float|Floor _m_shootingdamage))
    (else
      (bind _returnvalue_3 (Game|SpawnActorfromClass "/Game/Blueprints/Enemies/EnemyProjectile.EnemyProjectile_C" (Math|Transform|MakeTransform (+ _returnvalue (Math|Vector|RotateVector (Variables|Default|Getm_gunRotationOffset) _returnvalue_2)) (Class|KismetMathLibrary|MakeRot _pitch (Math|Random|RandomFloatinRange (- _yaw _m_shootingaccuracy) (+ _yaw _m_shootingaccuracy)) _roll) (Variables|Default|Getm_projectileScale)) true 0))
      (Variables|/Game/Blueprints/Enemies/EnemyProjectile.EnemyProjectile_C|Setm_collisionDamage _returnvalue_3 _m_shootingdamage)))
  (Audio|PlaySoundatLocation "/Game/Audio/Effects/EnemyShot_01_Cue.EnemyShot_01_Cue" _returnvalue))

(fn FacePlayerLockedZAxis
  (bind _returnvalue (Transformation|GetActorLocation))
  (bind _returnvalue_2 (Transformation|GetActorRotation))
  (bind _returnvalue_3 (Game|Player|GetPlayerPawn 0))
  (bind _returnvalue_4 (Transformation|GetActorLocation _returnvalue_3))
  ;[1 1 1] Rotate Toward player direction
  (if (<= (Math|Vector|VectorLength (- _returnvalue _returnvalue_4)) (Variables|Default|Getm_targetingDistance))
    (bind _asfirst_person_game_mode (Utilities|Casting|CastToFirstPersonGameMode (Game|GetGameMode)))
    (if (not (Variables|/Game/FirstPersonBP/Blueprints/FirstPersonGameMode.FirstPersonGameMode_C|Getm_playerDead _asfirst_person_game_mode))
      (Utilities|IsValid (Variables|/Game/FirstPersonBP/Blueprints/FirstPersonGameMode.FirstPersonGameMode_C|Getm_player _asfirst_person_game_mode)
        (:Is%20Valid
          (Utilities|IsValid (Game|Player|GetPlayerPawn 0)
            (:Is%20Valid
              (Transformation|SetActorRotation (Math|Interpolation|RInterpTo (Math|Rotator|MakeRotator (.pitch _returnvalue_2) (.yaw _returnvalue_2) (.roll _returnvalue_2)) (Math|Rotator|MakeRotator (.pitch _returnvalue_2) (.yaw (Math|Rotator|FindLookatRotation _returnvalue _returnvalue_4)) (.roll _returnvalue_2)) 0.1 0.5)))))))))