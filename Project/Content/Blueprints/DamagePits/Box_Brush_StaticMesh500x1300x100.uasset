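; Damage pit trigger volume that deals lethal-scale environment damage to the first-person player.
; A Box begin-overlap calls DamageActors, which applies EnviromentDamage equal to the character's max health, with the pit as damage causer.
; An overlap by an actor whose class is not exactly FirstPersonCharacter destroys the pit itself rather than the overlapping actor.
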(event OnComponentBeginOverlap(Box)
  (params (OtherActor :type Actor%20Object%20Reference) (OtherComp :type Primitive%20Component%20Object%20Reference) (OtherBodyIndex :type Integer) (bFromSweep :type Boolean) (SweepResult :type Hit%20Result%20Structure%20%28by%20ref%29))
  (CallFunction|DamageActors OtherActor))

(event EventBeginPlay)

(event EventActorBeginOverlap
  (params (OtherActor :type Actor%20Object%20Reference)))

(event EventTick
  (params (DeltaSeconds :type Float%20%28single-precision%29)))

(fn ConstructionScript)

(fn DamageActors
  (params (CollidedActor :type Actor%20Object%20Reference))
  (if (!= (Utilities|GetClass CollidedActor) "/Game/FirstPersonBP/Blueprints/FirstPersonCharacter.FirstPersonCharacter_C")
    (Actor|DestroyActor)
    (else
      (bind _asfirst_person_character (Utilities|Casting|CastToFirstPersonCharacter CollidedActor))
      (Game|Damage|ApplyDamage _asfirst_person_character (Math|Conversions|ToFloat(Integer) (Variables|/Game/FirstPersonBP/Blueprints/FirstPersonCharacter.FirstPersonCharacter_C|Getm_maxHealth _asfirst_person_character)) 0 self "/Game/Blueprints/EnviromentDamage.EnviromentDamage_C"))))